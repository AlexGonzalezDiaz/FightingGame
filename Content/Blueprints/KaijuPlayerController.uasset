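; Player controller for a kaiju fighting game that attempts to auto-face the opponent's controller toward a look-at target.
; BeginPlay caches the game mode and the player 0 third-person character.
; Tick prints the OtherPlayer controller's name and, past an IsValid check with no input, sets its yaw via RInterpTo.
; The look-at uses OtherPlayer's location as both start and target, so it never references the local character's position.
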(event `self.ReceiveBeginPlay`
  (bind _asfighting_game_game_mode_bp (cast `/Game/Dynamic/ThirdPerson/Blueprints/FightingGameGameMode_BP` (`GameplayStatics.GetGameMode`)))
  (set `self.As Fighting Game Game Mode BP` _asfighting_game_game_mode_bp)
  (bind _asbp_third_person_character (cast `/Game/Dynamic/ThirdPerson/Blueprints/BP_ThirdPersonCharacter` (`GameplayStatics.GetPlayerCharacter` 0)))
  (set `self.As BP Third Person Character` _asbp_third_person_character))

(event `self.ReceiveTick`
  (params (DeltaSeconds :type "Float (single-precision)"))
  (bind _otherplayer (`FightingGameCharacter.otherPlayer` (`self.As BP Third Person Character`)))
  (bind _returnvalue (`Pawn.GetController` _otherplayer))
  (bind (_returnvalue_roll _returnvalue_pitch _returnvalue_yaw) (`KismetMathLibrary.BreakRotator` (`KismetMathLibrary.RInterpTo` (`self.K2_GetActorRotation` _returnvalue) (`KismetMathLibrary.FindLookAtRotation` (`self.K2_GetActorLocation` _otherplayer) (`self.K2_GetActorLocation` _otherplayer)) (`GameplayStatics.GetWorldDeltaSeconds`) 20.0)))
  (`/Engine/EditorBlueprintResources/StandardMacros.IsValid` _otherplayer
    (:`Is Valid`
      (`KismetSystemLibrary.PrintString` (`KismetSystemLibrary.GetDisplayName` _returnvalue))
      (`/Engine/EditorBlueprintResources/StandardMacros.IsValid` null
        (:`Is Valid`
          (`self.SetControlRotation` _returnvalue (`KismetMathLibrary.MakeRotator` 0.0 0.0 _returnvalue_yaw)))))))

(fn `UserConstructionScript`)